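; PortalWall_BP is a wall for portal placement, with its mesh scaled from SizeWidth and SizeHeight in the construction script.
; SpawnPortal passes the hit point and PortalBlue's size to CheckPortal, leaving its IsPortalA branch empty.
; When the hit exceeds the positive Y or Z margin, MediatePortal offsets both coordinates using half-size margins and absolute values, then PortalBlue moves there.
; Hits within those limits move nothing, and the event graph is empty.
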(event EventBeginPlay)

(event Collision|EventActorBeginOverlap
  (params (OtherActor :type Actor%20Object%20Reference)))

(event EventTick
  (params (DeltaSeconds :type Float%20%28single-precision%29)))

(fn ConstructionScript
  (Transformation|SetWorldScale3D (Variables|Default|GetWall) (Math|Vector|MakeVector 1.0 (/ (Variables|Default|GetSizeWidth) 1e+02) (/ (Variables|Default|GetSizeHeight) 1e+02))))

(fn SpawnPortal
  (params (Is%20Portal%20A :type Boolean) (Hit%20Point :type Vector))
  (bind _portalblue (Variables|Default|GetPortalBlue))
  (CallFunction|CheckPortal Hit%20Point (Math|Vector|MakeVector 0.0 (Variables|/Game/PracticePT/Portal_Blue.Portal_Blue_C|GetSizeY _portalblue) (Variables|/Game/PracticePT/Portal_Blue.Portal_Blue_C|GetSizeZ _portalblue)))
  (if Is%20Portal%20A
    _))

(fn CheckPortal
  (params (Hit%20Point :type Vector) (Portal%20Size :type Vector))
  (if (> (.y Hit%20Point) (- (/ (Variables|Default|GetSizeWidth) 2.0) (.y Portal%20Size)))
    ;[1 1 1] 조정한 값을 포탈에 적용시킴
    (bind (_returny _returnz) (CallFunction|MediatePortal (.y Hit%20Point) (.z Hit%20Point) (.y Portal%20Size) (.z Portal%20Size) :!label _label))
    (Transformation|SetActorLocation (Variables|Default|GetPortalBlue) (Math|Vector|MakeVector 0.0 _returny _returnz) false false)
    (elif (> (.z Hit%20Point) (- (/ (Variables|Default|GetSizeHeight) 2.0) (.z Portal%20Size)))
      (goto _label))))

(fn MediatePortal
  (params (locationY :type Float%20%28single-precision%29) (LocationZ :type Float%20%28single-precision%29) (PortalRadiusY :type Float%20%28single-precision%29) (PortalRadiusZ :type Float%20%28single-precision%29))
  ;[1 1 1] y좌표 조정
  ;;[1 1 1] 좌표 양 저장
  (LocalVariables|SetAmountY (- (- (/ (Variables|Default|GetSizeWidth) 2.0) PortalRadiusY) (Math|Float|Absolute(Float) locationY)))
  ;;[1 1 1] New 좌표 저장
  (LocalVariables|SetAmountY (+ (LocalVariables|GetAmountY) locationY))
  ;[1 1 1] z좌표 조정
  (LocalVariables|SetAmountZ (- (- (/ (Variables|Default|GetSizeHeight) 2.0) PortalRadiusZ) (Math|Float|Absolute(Float) LocationZ)))
  (LocalVariables|SetAmountZ (+ (LocalVariables|GetAmountZ) LocationZ))
  (return (LocalVariables|GetAmountY) (LocalVariables|GetAmountZ)))